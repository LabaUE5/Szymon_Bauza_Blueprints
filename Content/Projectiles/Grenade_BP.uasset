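; Grenade projectile that explodes on a fixed timer after spawning.
; BeginPlay waits a short delay, then spawns an explosion emitter at the mesh, fires a radial force impulse, plays the blast sound and destroys the actor.
; Hits on the static mesh play a bounce sound at its location.
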(event OnComponentHit(StaticMesh)
  (params (HitComponent :type Primitive%20Component%20Object%20Reference) (OtherActor :type Actor%20Object%20Reference) (OtherComp :type Primitive%20Component%20Object%20Reference) (NormalImpulse :type Vector :default "0, 0, 0") (Hit :type Hit%20Result%20Structure%20%28by%20ref%29))
  (Audio|PlaySoundatLocation "/Game/Projectiles/Grenade_bounce.Grenade_bounce" (Transformation|GetWorldLocation (Variables|Default|GetStaticMesh)) "0, 0, 0" 1.0 1.0 0.0 0 0 0 0))

(event EventBeginPlay
  (Utilities|FlowControl|Delay 2.0)
  (Effects|SpawnEmitteratLocation "/Game/Realistic_Starter_VFX_Pack_Vol2/Particles/Explosion/P_Explosion_Big_A.P_Explosion_Big_A" (Transformation|GetWorldLocation (Variables|Default|GetStaticMesh)))
  (Class|RadialForceComponent|FireImpulse (Variables|Default|GetRadialForce))
  (Audio|PlaySoundatLocation "/Game/Projectiles/Grenade_explosion.Grenade_explosion" (Transformation|GetWorldLocation (Variables|Default|GetStaticMesh)) "0, 0, 0" 1.0 1.0 0.0 0 0 0 0)
  (Actor|DestroyActor))

(fn ConstructionScript)